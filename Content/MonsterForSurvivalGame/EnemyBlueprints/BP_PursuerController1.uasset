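; AI controller for Pursuer enemies in a survival game that chases the player and attacks at close range.
; Every tick it compares player distance with AttackRange and time since the last attack with AttackCooldown.
; When both pass it calls PlayAttack on the pawn, trying a BP_Pursuer1 cast before BP_Pursuer.
; Otherwise it reissues AI MoveTo toward player 0, even when in range during cooldown.
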(event `TryAttack`
  (bind _asbp_pursuer_1 (cast `/Game/MonsterForSurvivalGame/EnemyBlueprints/BP_Pursuer1` (`self.K2_GetPawn`))
    (:`then`
      (`/Game/MonsterForSurvivalGame/EnemyBlueprints/BP_Pursuer1.PlayAttack` _asbp_pursuer_1))
    (:`CastFailed`
      (bind _asbp_pursuer (cast `/Game/MonsterForSurvivalGame/EnemyBlueprints/BP_Pursuer` (`self.K2_GetPawn`)))
      (`/Game/MonsterForSurvivalGame/EnemyBlueprints/BP_Pursuer.PlayAttack` _asbp_pursuer))))

(event `self.ReceiveTick`
  (params (DeltaSeconds :type "Float (single-precision)"))
  (if (and (<= (`KismetMathLibrary.Vector_Distance` (`self.K2_GetActorLocation` (`GameplayStatics.GetPlayerCharacter` 0)) (`self.K2_GetActorLocation` (`self.K2_GetPawn`))) (`self.attackRange`)) (> (- (`KismetSystemLibrary.GetGameTimeInSeconds`) (`self.LastAttackTime`)) (`self.AttackCooldown`)))
    (set `self.LastAttackTime` (`KismetSystemLibrary.GetGameTimeInSeconds`))
    (`self.TryAttack`)
    (else
      (`self.StartChasingPlayer`))))

(event `StartChasingPlayer`
  (`|AIMoveTo` (`self.K2_GetPawn`) (0.0 0.0 0.0) (`GameplayStatics.GetPlayerCharacter` 0) 75.0 true))

(fn `UserConstructionScript`)