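; Pursuer enemy for a survival game, with a boosted walk speed, its own health and a damage attack on the player.
; Incoming damage lowers health and briefly sets a hit flag; at zero health it calls Die.
; Die always drops a coin, rolls in sequence for one bonus magnet, health pack or buff, increments player score, then destroys the actor.
; PlayAttack damages the player, scaled inversely by their DEF stat.
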(event `self.ReceiveBeginPlay`
  (set `self.Health_0` (`self.Health`))
  (set `CharacterMovementComponent.MaxWalkSpeed` 700.0 (`self.CharacterMovement`)))

(event `self.ReceiveAnyDamage`
  (params (Damage :type "Float (single-precision)") (DamageType :type "DamageType Object Reference") (InstigatedBy :type "Controller Object Reference") (DamageCauser :type "Actor Object Reference"))
  (if (not (`self.bIsDead`))
    (bind _output_get (set `self.Health_0` (`KismetMathLibrary.FMax` (- (`self.Health_0`) Damage))))
    (set `self.bIsHit` true)
    (if (<= _output_get 0.0)
      (set `self.bIsDead` true)
      (`self.Die`)
      (else
        (`KismetSystemLibrary.Delay` 0.5)
        (set `self.bIsHit` false)))))

(event `Die`
  (bind _returnvalue (`self.GetTransform`))
  (bind _returnvalue_2 (`KismetMathLibrary.RandomInteger` 100))
  (bind _returnvalue_3 (+ (.x (.location _returnvalue)) 50.0))
  (set `self.bIsHit` false)
  (set `self.bIsAttacking` false)
  (`CharacterMovementComponent.DisableMovement` (`self.CharacterMovement`))
  (`|SpawnActorFromClass` "/Game/VisualSandbox/Blueprints/Pickups/Drop_Out/BP_Coin.BP_Coin_C" (`self.GetTransform`) "Undefined" "MultiplyWithRoot" null null)
  (if (> _returnvalue_2 80)
    (`|SpawnActorFromClass` "/Game/VisualSandbox/Blueprints/Pickups/Drop_Out/BP_Magnet.BP_Magnet_C" (`KismetMathLibrary.MakeTransform` (`KismetMathLibrary.MakeVector` _returnvalue_3 (.y (.location _returnvalue)) (.z (.location _returnvalue))) (.rotation _returnvalue) (.scale _returnvalue)) "Undefined" "MultiplyWithRoot" null null)
    (elif (> _returnvalue_2 80)
      (`|SpawnActorFromClass` "/Game/VisualSandbox/Blueprints/Pickups/Drop_Out/BP_Health_Pack.BP_Health_Pack_C" (`KismetMathLibrary.MakeTransform` (`KismetMathLibrary.MakeVector` _returnvalue_3 (.y (.location _returnvalue)) (.z (.location _returnvalue))) (.rotation _returnvalue) (.scale _returnvalue)) "Undefined" "MultiplyWithRoot" null null)
      (elif (> _returnvalue_2 80)
        (`|SpawnActorFromClass` "/Game/VisualSandbox/Blueprints/Pickups/Drop_Out/BP_Buff.BP_Buff_C" (`KismetMathLibrary.MakeTransform` (`KismetMathLibrary.MakeVector` _returnvalue_3 (.y (.location _returnvalue)) (.z (.location _returnvalue))) (.rotation _returnvalue) (.scale _returnvalue)) "Undefined" "MultiplyWithRoot" null null))))
  (bind _asbp_third_person_pawn (cast `/Game/VisualSandbox/Blueprints/GameModes/ThirdPerson/BP_ThirdPerson_Pawn` (`GameplayStatics.GetPlayerPawn` 0)))
  (set `/Game/VisualSandbox/Blueprints/GameModes/ThirdPerson/BP_ThirdPerson_Pawn.Score` (+ (`/Game/VisualSandbox/Blueprints/GameModes/ThirdPerson/BP_ThirdPerson_Pawn.Score` _asbp_third_person_pawn) 1) _asbp_third_person_pawn)
  (`self.K2_DestroyActor`))

(event `PlayAttack`
  (bind _asbp_third_person_pawn (cast `/Game/VisualSandbox/Blueprints/GameModes/ThirdPerson/BP_ThirdPerson_Pawn` (`GameplayStatics.GetPlayerCharacter` 0)))
  (`GameplayStatics.ApplyDamage` (`GameplayStatics.GetPlayerCharacter` 0) (/ (`self.Damage`) (/ (`/Game/VisualSandbox/Blueprints/GameModes/ThirdPerson/BP_ThirdPerson_Pawn.DEF` _asbp_third_person_pawn) 100.0)))
  (`KismetSystemLibrary.PrintString` "attempt to deal damage"))

(fn `UserConstructionScript`)