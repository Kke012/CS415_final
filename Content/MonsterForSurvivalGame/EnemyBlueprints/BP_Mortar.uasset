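; BP_Mortar is a survival-game enemy that lobs shells at the player and drops pickups when killed.
; PlayAttack uses SuggestProjectileVelocity to compute an arc toward a point slightly offset from the player, then spawns a BP_MortarShell with that velocity and its damage.
; AnyDamage lowers health and briefly sets a hit flag.
; Death disables movement, spawns a coin and possibly a magnet, health pack or buff through chained random rolls, then destroys the actor.
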(event `self.ReceiveBeginPlay`
  (set `self.Health_0` (`self.Health`)))

(event `self.ReceiveAnyDamage`
  (params (Damage :type "Float (single-precision)") (DamageType :type "DamageType Object Reference") (InstigatedBy :type "Controller Object Reference") (DamageCauser :type "Actor Object Reference"))
  (if (not (`self.bIsDead`))
    (bind _output_get (set `self.Health_0` (`KismetMathLibrary.FMax` (- (`self.Health_0`) Damage))))
    (set `self.bIsHit` true)
    (if (<= _output_get 0.0)
      (set `self.bIsDead` true)
      (`self.Die`)
      (else
        (`KismetSystemLibrary.Delay` 0.5)
        (set `self.bIsHit` false)))))

(event `Die`
  (bind _returnvalue (`self.GetTransform`))
  (bind _returnvalue_2 (`KismetMathLibrary.RandomInteger` 100))
  (bind _returnvalue_3 (+ (.x (.location _returnvalue)) 50.0))
  (set `self.bIsHit` false)
  (set `self.bIsAttacking` false)
  (`CharacterMovementComponent.DisableMovement` (`self.CharacterMovement`))
  (`|SpawnActorFromClass` "/Game/VisualSandbox/Blueprints/Pickups/Drop_Out/BP_Coin.BP_Coin_C" (`self.GetTransform`) "Undefined" "MultiplyWithRoot" null null)
  (if (> _returnvalue_2 80)
    (`|SpawnActorFromClass` "/Game/VisualSandbox/Blueprints/Pickups/Drop_Out/BP_Magnet.BP_Magnet_C" (`KismetMathLibrary.MakeTransform` (`KismetMathLibrary.MakeVector` _returnvalue_3 (.y (.location _returnvalue)) (.z (.location _returnvalue))) (.rotation _returnvalue) (.scale _returnvalue)) "Undefined" "MultiplyWithRoot" null null)
    (elif (> _returnvalue_2 90)
      (`|SpawnActorFromClass` "/Game/VisualSandbox/Blueprints/Pickups/Drop_Out/BP_Health_Pack.BP_Health_Pack_C" (`KismetMathLibrary.MakeTransform` (`KismetMathLibrary.MakeVector` _returnvalue_3 (.y (.location _returnvalue)) (.z (.location _returnvalue))) (.rotation _returnvalue) (.scale _returnvalue)) "Undefined" "MultiplyWithRoot" null null)
      (elif (> _returnvalue_2 95)
        (`|SpawnActorFromClass` "/Game/VisualSandbox/Blueprints/Pickups/Drop_Out/BP_Buff.BP_Buff_C" (`KismetMathLibrary.MakeTransform` (`KismetMathLibrary.MakeVector` _returnvalue_3 (.y (.location _returnvalue)) (.z (.location _returnvalue))) (.rotation _returnvalue) (.scale _returnvalue)) "Undefined" "MultiplyWithRoot" null null))))
  (`self.K2_DestroyActor`))

(event `PlayAttack`
  (bind _arrow1 (`self.Arrow1`))
  (bind _returnvalue (`SceneComponent.K2_GetComponentLocation` _arrow1))
  (bind (_tossvelocity _returnvalue_2) (`GameplayStatics.BlueprintSuggestProjectileVelocity` _returnvalue (+ (`self.K2_GetActorLocation` (`GameplayStatics.GetPlayerPawn` 0)) (0.0 50.0 0.0)) 2000.0 0.0 "DoNotTrace"))
  (if _returnvalue_2
    (bind _returnvalue_3 (`|SpawnActorFromClass` "/Game/MonsterForSurvivalGame/EnemyBlueprints/BP_MortarShell.BP_MortarShell_C" (`KismetMathLibrary.MakeTransform` _returnvalue (`SceneComponent.K2_GetComponentRotation` _arrow1)) "Undefined" "MultiplyWithRoot" self 100.0 (`self.Damage`) null))
    (set `MovementComponent.Velocity` _tossvelocity (`/Game/MonsterForSurvivalGame/EnemyBlueprints/BP_MortarShell.ProjectileMovement` _returnvalue_3))))

(fn `UserConstructionScript`)