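; BP_MortarShell is a mortar shell projectile that deals radial damage on contact, ignoring its owner.
; A Sphere overlap applies fixed damage around the shell's location, then destroys the actor.
; A Sphere hit instead applies the Damage variable around the impact point and leaves the shell alive.
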(event `self.Sphere.OnComponentBeginOverlap`
  (params (OverlappedComponent :type "PrimitiveComponent Object Reference") (OtherActor :type "Actor Object Reference") (OtherComp :type "PrimitiveComponent Object Reference") (OtherBodyIndex :type Integer) (bFromSweep :type Boolean) (SweepResult :type "HitResult Structure (by ref)"))
  (if (not (== OtherActor (`self.GetOwner`)))
    (`GameplayStatics.ApplyRadialDamage` :`BaseDamage` 50.0 :`Origin` (`self.K2_GetActorLocation`) :`DamageRadius` 500.0 :`DamageCauser` null :`InstigatedByController` null)
    (`self.K2_DestroyActor`)))

(event `self.Sphere.OnComponentHit`
  (params (HitComponent :type "PrimitiveComponent Object Reference") (OtherActor :type "Actor Object Reference") (OtherComp :type "PrimitiveComponent Object Reference") (NormalImpulse :type "Vector Structure") (Hit :type "HitResult Structure (by ref)"))
  (if (not (== OtherActor (`self.GetOwner`)))
    (`GameplayStatics.ApplyRadialDamage` :`BaseDamage` (`self.Damage`) :`Origin` (`.Location` (`GameplayStatics.BreakHitResult` Hit)) :`DamageRadius` 500.0 :`DamageCauser` null :`InstigatedByController` null)))

(fn `UserConstructionScript`)