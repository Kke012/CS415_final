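; AI controller for Pursuer and Mortar enemies that roam around their spawn point, chase the player once seen, and attack within range.
; Pawn sensing starts the chase and a looping line-of-sight timer, which returns the enemy to roaming after a grace period without sight.
; Tick gates attacks by distance and cooldown, with Mortars getting longer range and stopping movement before firing.
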(event `StartRoaming`
  (if (not (`self.bHasSeenPlayer`))
    (`|AIMoveTo` (`self.K2_GetPawn`) (`NavigationSystemV1.K2_GetRandomReachablePointInRadius` (`self.Home location`) (`self.RoamRadius`) null null) null 100.0
      (:`then`
        (`KismetSystemLibrary.Delay` 1.0)
        (`self.StartRoaming`)))))

(event `self.ReceiveBeginPlay`
  (bind _returnvalue (`self.K2_GetPawn`))
  (set `self.Home location` (`self.K2_GetActorLocation` _returnvalue))
  (cast `/Game/MonsterForSurvivalGame/EnemyBlueprints/BP_Mortar` _returnvalue
    (:`then`
      (set `self.attackRange` 2000.0))
    (:`CastFailed`
      _))
  (`self.StartRoaming`))

(event `TryAttack`
  (bind _asbp_pursuer (cast `/Game/MonsterForSurvivalGame/EnemyBlueprints/BP_Pursuer` (`self.K2_GetPawn`))
    (:`then`
      (`/Game/MonsterForSurvivalGame/EnemyBlueprints/BP_Pursuer.PlayAttack` _asbp_pursuer))
    (:`CastFailed`
      (bind _asbp_mortar (cast `/Game/MonsterForSurvivalGame/EnemyBlueprints/BP_Mortar` (`self.K2_GetPawn`)))
      (`self.StopMovement`)
      (`/Game/MonsterForSurvivalGame/EnemyBlueprints/BP_Mortar.PlayAttack` _asbp_mortar))))

(event `self.ReceiveTick`
  (params (DeltaSeconds :type "Float (single-precision)"))
  (if (`self.bHasSeenPlayer`)
    (if (and (<= (`KismetMathLibrary.Vector_Distance` (`self.K2_GetActorLocation` (`self.TargetActor`)) (`self.K2_GetActorLocation` (`self.K2_GetPawn`))) (`self.attackRange`)) (> (- (`KismetSystemLibrary.GetGameTimeInSeconds`) (`self.LastAttackTime`)) (`self.AttackCooldown`)))
      (set `self.LastAttackTime` (`KismetSystemLibrary.GetGameTimeInSeconds`))
      (`self.TryAttack`)
      (else
        (`self.StartChasingPlayer`)))))

(event `self.PawnSensing.OnSeePawn`
  (params (Pawn :type "Pawn Object Reference"))
  (if (`self.bHasSeenPlayer`)
    (`self.StartChasingPlayer`)
    (else
      (set `self.bHasSeenPlayer` true)
      (set `self.TargetActor` (`GameplayStatics.GetPlayerCharacter` 0))
      (`self.StartChasingPlayer`)))
  (set `self.LastSeenTime` (`KismetSystemLibrary.GetGameTimeInSeconds`))
  (`KismetSystemLibrary.K2_ClearAndInvalidateTimerHandle` (`self.CheckSightTimer`))
  (bind _returnvalue (`KismetSystemLibrary.K2_SetTimerDelegate` (delegate `CheckSIght`) 0.1 true))
  (set `self.CheckSightTimer` _returnvalue))

(event `CheckSIght`
  (bind _returnvalue (`KismetSystemLibrary.GetGameTimeInSeconds`))
  (if (`self.LineOfSightTo` (`GameplayStatics.GetPlayerCharacter` 0))
    (set `self.LastSeenTime` _returnvalue)
    (elif (>= (- _returnvalue (`self.LastSeenTime`)) (`self.LoseSightGrace`))
      (`KismetSystemLibrary.K2_ClearAndInvalidateTimerHandle` (`self.CheckSightTimer`))
      (set `self.bHasSeenPlayer` false)
      (`self.StartRoaming`))))

(event `StartChasingPlayer`
  (`|AIMoveTo` (`self.K2_GetPawn`) (0.0 0.0 0.0) (`self.TargetActor`) 75.0 true))

(fn `UserConstructionScript`)