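; BP_Buff_Store is a prop actor whose Beam component acts as a distance-dependent visual for the buff store.
; Every Tick it measures the distance to player pawn 0 and shows the Beam at or beyond BeamShowDistance, hiding it when closer.
; Showing propagates to the Beam's child components, while hiding affects only the Beam itself.
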(event `self.ReceiveTick`
  (params (DeltaSeconds :type "Float (single-precision)"))
  (if (>= (`KismetMathLibrary.VSize` (- (`self.K2_GetActorLocation`) (`self.K2_GetActorLocation` (`GameplayStatics.GetPlayerPawn` 0)))) (`self.BeamShowDistance`))
    (`SceneComponent.SetVisibility` (`self.Beam`) true true)
    (else
      (`SceneComponent.SetVisibility` (`self.Beam`) false false))))

(fn `UserConstructionScript`)