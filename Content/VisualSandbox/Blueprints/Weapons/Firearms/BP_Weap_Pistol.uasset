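; BP_Weap_Pistol is a pistol firearm Blueprint that defines how the weapon improves when it levels up.
; LevelUp, while below MaxLevel, raises the level, rate of fire, damage and magazine capacity by fixed steps, then refills the rounds.
; The event graph holds only disabled default events, and the construction script just calls its parent.
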(fn `LevelUp`
  (if (< (`self.Level`) (`self.MaxLevel`))
    (set `self.Level` (+ (`self.Level`) 1))
    (set `self.Rate Of Fire` (+ (`self.Rate Of Fire`) 25.0))
    (set `self.Weapon Damage` (+ (`self.Weapon Damage`) 10.0))
    (set `self.Max Rounds` (+ (`self.Max Rounds`) 2))
    (set `self.Rounds` (`self.Max Rounds`))))

(fn `UserConstructionScript`
  (`parent.UserConstructionScript`))