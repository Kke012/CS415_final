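; BP_Round_Manager runs a level's timed enemy rounds, from pre-round countdown to end-of-level handling.
; Timers chain StartNextRound, BeginRound and EndRound, showing countdown widgets and starting or stopping every BP_Enemy_Spawner.
; EndRound destroys enemies and boss health UI, then spawns a buff store between rounds.
; After the final round it spawns a weapon store and next-level portal, or shows a paused completion screen on the last level.
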(event `self.ReceiveBeginPlay`
  (bind _outactors (`GameplayStatics.GetAllActorsOfClass` "/Game/VisualSandbox/Blueprints/Game/BP_Enemy_Spawner.BP_Enemy_Spawner_C"))
  (set `self.AllSpawners` _outactors)
  (set `self.CurrentRound` 0)
  (`self.StartNextRound`))

(event `StartNextRound`
  (set `self.Spawned` false)
  (set `self.CurrentRound` (+ (`self.CurrentRound`) 1))
  (if (<= (`self.CurrentRound`) (`self.MaxRound`))
    (`GameplayStatics.PlaySound2D` "/Engine/EngineSounds/1kSineTonePing.1kSineTonePing" 1.0 1.0 0.0 null null)
    (bind _returnvalue (`|CreateWidget` "/Game/VisualSandbox/Blueprints/UMG/CountDown/WBP_Count_Down.WBP_Count_Down_C" null (`self.PreRoundDuration`)))
    (`UserWidget.AddToViewport` _returnvalue 0)
    (`KismetSystemLibrary.K2_SetTimer` null "BeginRound" (`KismetMathLibrary.Conv_IntToDouble` (`self.PreRoundDuration`)))))

(event `BeginRound`
  (`GameplayStatics.PlaySound2D` "/Game/game_item/Destruction/Destructionsoundsw6.Destructionsoundsw6" 1.0 1.0 0.0 null null)
  (bind _returnvalue (`|CreateWidget` "/Game/VisualSandbox/Blueprints/UMG/CountDown/WBP_Count_Down.WBP_Count_Down_C" null (`self.RoundDuration`)))
  (`UserWidget.AddToViewport` _returnvalue 0)
  (bind _returnvalue_2 (`KismetSystemLibrary.K2_SetTimer` null "EndRound" (`KismetMathLibrary.Conv_IntToDouble` (`self.RoundDuration`))))
  (set `self.RoundTimerHandler` _returnvalue_2)
  (for _array_element (`self.AllSpawners`)
    (`/Game/VisualSandbox/Blueprints/Game/BP_Enemy_Spawner.StartSpawning` _array_element (`self.CurrentRound`))))

(event `EndRound`
  (bind _returnvalue (`self.GetTransform`))
  (`KismetSystemLibrary.K2_ClearAndInvalidateTimerHandle` (`self.RoundTimerHandler`))
  (for _array_element (`self.AllSpawners`)
    (`/Game/VisualSandbox/Blueprints/Game/BP_Enemy_Spawner.StopSpawning` _array_element)
    (bind _outactors (`GameplayStatics.GetAllActorsOfClass` "/Game/VisualSandbox/Blueprints/Game/BP_Enemy.BP_Enemy_C"))
    (for _array_element_2 _outactors
      (bind _asbp_boss (cast `/Game/VisualSandbox/Blueprints/Boss/BP_Boss` _array_element_2)
        (:`then`
          (`Widget.RemoveFromParent` (`/Game/VisualSandbox/Blueprints/Boss/BP_Boss.HealthUI` _asbp_boss)))
        (:`CastFailed`
          (bind _asbp_boss_2 (cast `/Game/VisualSandbox/Blueprints/Boss/BP_Boss2` _array_element_2)
            (:`then`
              (`Widget.RemoveFromParent` (`/Game/VisualSandbox/Blueprints/Boss/BP_Boss2.Health UI2` _asbp_boss_2)))
            (:`CastFailed`
              _))))
      (`self.K2_DestroyActor` _array_element_2))
    (if (not (`self.Spawned`))
      (set `self.Spawned` true)
      (if (< (`self.CurrentRound`) (`self.MaxRound`))
        (`|SpawnActorFromClass` "/Game/VisualSandbox/Blueprints/Props/BP_Buff_Store.BP_Buff_Store_C" (`self.GetTransform`) "Undefined" "MultiplyWithRoot" null null)
        (elif (`self.LastLevel`)
          (`GameplayStatics.PlaySound2D` "/Game/game_item/Drop/BouncyRubberBall8.BouncyRubberBall8" 1.0 1.0 0.0 null null)
          (bind _returnvalue_2 (`|CreateWidget` "/Game/VisualSandbox/Blueprints/UMG/Common/WBP_Complete.WBP_Complete_C"))
          (`UserWidget.AddToViewport` _returnvalue_2 0)
          (`GameplayStatics.SetGamePaused` true)
          (set `PlayerController.bShowMouseCursor` true (`GameplayStatics.GetPlayerController` 0))
          (`WidgetBlueprintLibrary.SetInputMode_UIOnlyEx` (`GameplayStatics.GetPlayerController` 0) null "DoNotLock" true)
          (else
            (`|SpawnActorFromClass` "/Game/VisualSandbox/Blueprints/Props/BP_Weapon_Store.BP_Weapon_Store_C" (`self.GetTransform`) "Undefined" "MultiplyWithRoot" null null)
            (`|SpawnActorFromClass` "/Game/VisualSandbox/Blueprints/Props/BP_Level_Portal.BP_Level_Portal_C" (`KismetMathLibrary.MakeTransform` (`KismetMathLibrary.MakeVector` (+ (.x (.location _returnvalue)) 120.0) (.y (.location _returnvalue)) (.z (.location _returnvalue))) (.rotation _returnvalue) (.scale _returnvalue)) "Undefined" "MultiplyWithRoot" null (`self.NextLevel`) null)))))))

(fn `UserConstructionScript`)