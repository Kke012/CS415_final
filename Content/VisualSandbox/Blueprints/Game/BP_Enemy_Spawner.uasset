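; BP_Enemy_Spawner is an actor that spawns enemies at its own transform during rounds.
; StartSpawning takes a round number and, once it reaches RoundsToActivate, starts a looping timer at SpawnInterval that calls SpawnOnce.
; SpawnOnce spawns the configured EnemyClass, passing in the spawner's Health and Damage values.
; StopSpawning clears the timer, and the spawner does nothing on its own at BeginPlay or Tick.
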(event `StartSpawning`
  (params (RoundNumber :type Integer))
  (if (>= RoundNumber (`self.RoundsToActivate`))
    (`KismetSystemLibrary.K2_SetTimer` null "SpawnOnce" (`self.SpawnInterval`) true)))

(event `SpawnOnce`
  (`|SpawnActorFromClass` (`self.EnemyClass`) (`self.GetTransform`) "Undefined" "MultiplyWithRoot" null (`self.Health`) (`self.Damage`) null))

(event `StopSpawning`
  (`KismetSystemLibrary.K2_ClearTimer` null "SpawnOnce"))

(fn `UserConstructionScript`)