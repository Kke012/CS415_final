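; Boss enemy that fights the player with ranged wave projectiles, random teleports and an on-screen health bar.
; A looping timer turns it toward a player in range and randomly fires either a stun wave or a damage wave scaled by player DEF.
; A second timer shifts it randomly around its current position, drifting only upward in Z.
; On death it drops a gold coin, adds score and destroys itself.
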(event `DoStunAttack`
  (bind _projectilespawnpoint (`self.ProjectileSpawnPoint`))
  (bind _returnvalue (`SceneComponent.K2_GetComponentLocation` _projectilespawnpoint))
  ; Attack
  (`GameplayStatics.PlaySoundAtLocation` "/Game/FreeModularMagicSFX/D1_Spell/Stereo/SW_Stereo_MagicWeapon_Summon_1.SW_Stereo_MagicWeapon_Summon_1" _returnvalue (struct) 1.0 1.0 0.0 null null null null)
  (bind _returnvalue_2 (`|SpawnActorFromClass` (`self.CCProjectileClass`) (`KismetMathLibrary.MakeTransform` _returnvalue (`SceneComponent.K2_GetComponentRotation` _projectilespawnpoint)) "AdjustIfPossibleButAlwaysSpawn" "MultiplyWithRoot" null null))
  (bind _asbp_wave_cc (cast `/Game/VisualSandbox/Blueprints/Projectiles/BP_Wave_CC` _returnvalue_2))
  (set `/Game/VisualSandbox/Blueprints/Projectiles/BP_Wave_CC.StunDuration` 0.75 _asbp_wave_cc))

(event `DoDamageAttack`
  (bind _projectilespawnpoint (`self.ProjectileSpawnPoint`))
  (bind _returnvalue (`SceneComponent.K2_GetComponentLocation` _projectilespawnpoint))
  ; Attack
  (`GameplayStatics.PlaySoundAtLocation` "/Game/FreeModularMagicSFX/D1_Spell/Stereo/SW_Stereo_MagicWeapon_Summon_1.SW_Stereo_MagicWeapon_Summon_1" _returnvalue (struct) 1.0 1.0 0.0 null null null null)
  (bind _returnvalue_2 (`|SpawnActorFromClass` (`self.DamageProjectileClass`) (`KismetMathLibrary.MakeTransform` _returnvalue (`SceneComponent.K2_GetComponentRotation` _projectilespawnpoint)) "AdjustIfPossibleButAlwaysSpawn" "MultiplyWithRoot" null null))
  (bind _asbp_wave_damage (cast `/Game/VisualSandbox/Blueprints/Projectiles/BP_Wave_Damage` _returnvalue_2))
  (bind _asbp_third_person_pawn (cast `/Game/VisualSandbox/Blueprints/GameModes/ThirdPerson/BP_ThirdPerson_Pawn` (`GameplayStatics.GetPlayerPawn` 0)))
  (set `/Game/VisualSandbox/Blueprints/Projectiles/BP_Wave_Damage.DamageAmount` (/ (`self.Damage`) (/ (`/Game/VisualSandbox/Blueprints/GameModes/ThirdPerson/BP_ThirdPerson_Pawn.DEF` _asbp_third_person_pawn) 100.0)) _asbp_wave_damage))

(event `BossAttackTick`
  (bind _returnvalue (`self.K2_GetActorLocation`))
  ; Attack
  (bind _asbp_third_person_pawn (cast `/Game/VisualSandbox/Blueprints/GameModes/ThirdPerson/BP_ThirdPerson_Pawn` (`GameplayStatics.GetPlayerCharacter` 0)))
  (bind _returnvalue_2 (`self.K2_GetActorLocation` _asbp_third_person_pawn))
  (if (<= (`KismetMathLibrary.Vector_Distance` _returnvalue _returnvalue_2) (`self.AttackRange`))
    (`self.K2_SetActorRotation` (`KismetMathLibrary.FindLookAtRotation` _returnvalue _returnvalue_2))
    (if (== (`KismetMathLibrary.RandomIntegerInRange` 0 1) 0)
      (`self.DoDamageAttack`)
      (else
        (`self.DoStunAttack`)))))

(event `self.ReceiveBeginPlay`
  ; Health UI
  (set `self.maxHealth` (`self.Health`))
  (bind _returnvalue (`|CreateWidget` "/Game/VisualSandbox/Blueprints/Boss/WB_Boss_Health.WB_Boss_Health_C"))
  (`UserWidget.AddToViewport` _returnvalue 0)
  (set `self.Health UI2` _returnvalue)
  (`KismetSystemLibrary.K2_SetTimer` null "BossAttackTick" (`self.AttackInterval`) true)
  (`KismetSystemLibrary.K2_SetTimer` null "BossTeleportTick" (`self.TeleportInterval`) true))

(event `self.ReceiveTick`
  (params (DeltaSeconds :type "Float (single-precision)"))
  ; Health UI
  (`ProgressBar.SetPercent` (`/Game/VisualSandbox/Blueprints/Boss/WB_Boss_Health.Health_Bar` (`self.Health UI2`)) (/ (`self.Health`) (`self.maxHealth`))))

(event `BossTeleportTick`
  ; TP
  (`self.K2_SetActorLocation` (`KismetMathLibrary.MakeVector` (+ (.x (`self.K2_GetActorLocation`)) (`KismetMathLibrary.RandomFloatInRange` (* (`self.TeleportRadius`) -1.0) (`self.TeleportRadius`))) (+ (.y (`self.K2_GetActorLocation`)) (`KismetMathLibrary.RandomFloatInRange` (* (`self.TeleportRadius`) -1.0) (`self.TeleportRadius`))) (+ (.z (`self.K2_GetActorLocation`)) (`KismetMathLibrary.RandomFloatInRange` 0.0 75.0))) true))

(event `self.ReceiveAnyDamage`
  (params (Damage :type "Float (single-precision)") (DamageType :type "DamageType Object Reference") (InstigatedBy :type "Controller Object Reference") (DamageCauser :type "Actor Object Reference"))
  ; Health
  (set `self.Health` (- (`self.Health`) Damage))
  (if (<= (`self.Health`) 0.0)
    (`CharacterMovementComponent.DisableMovement` (`self.CharacterMovement`))
    (`PrimitiveComponent.SetSimulatePhysics` (`self.Mesh`) true)
    (`Widget.RemoveFromParent` (`self.Health UI2`))
    (`|SpawnActorFromClass` "/Game/VisualSandbox/Blueprints/Pickups/Drop_Out/BP_GoldCoin.BP_GoldCoin_C" (`self.GetTransform`) "Undefined" "MultiplyWithRoot" null null)
    (bind _asbp_third_person_pawn (cast `/Game/VisualSandbox/Blueprints/GameModes/ThirdPerson/BP_ThirdPerson_Pawn` (`GameplayStatics.GetPlayerPawn` 0)))
    (set `/Game/VisualSandbox/Blueprints/GameModes/ThirdPerson/BP_ThirdPerson_Pawn.Score` (+ (`/Game/VisualSandbox/Blueprints/GameModes/ThirdPerson/BP_ThirdPerson_Pawn.Score` _asbp_third_person_pawn) 10) _asbp_third_person_pawn)
    (`self.K2_DestroyActor`)))

(fn `UserConstructionScript`)