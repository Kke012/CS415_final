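; Boss enemy character with health, a screen health bar and a montage-driven magic attack.
; Damage lowers health; at zero it stops movement, ragdolls the mesh and flags death, while Tick feeds the health widget.
; Attack plays a Beholder montage unless busy or dead; its notify sphere-traces forward for pawns, applies damage, and fires camera shake, Niagara effect and sound.
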(event `self.ReceiveAnyDamage`
  (params (Damage :type "Float (single-precision)") (DamageType :type "DamageType Object Reference") (InstigatedBy :type "Controller Object Reference") (DamageCauser :type "Actor Object Reference"))
  ; Health
  (set `self.Health` (- (`self.Health`) Damage))
  (if (<= (`self.Health`) 0.0)
    (`CharacterMovementComponent.DisableMovement` (`self.CharacterMovement`))
    (`PrimitiveComponent.SetSimulatePhysics` (`self.Mesh`) true)
    (set `self.isDead?` true)))

(event `self.ReceiveBeginPlay`
  (bind _returnvalue (`|CreateWidget` "/Game/VisualSandbox/Blueprints/Boss/WB_Boss_Health.WB_Boss_Health_C"))
  (`UserWidget.AddToViewport` _returnvalue 0)
  (set `self.HealthUI` _returnvalue))

(event `self.ReceiveTick`
  (params (DeltaSeconds :type "Float (single-precision)"))
  (`ProgressBar.SetPercent` (`/Game/VisualSandbox/Blueprints/Boss/WB_Boss_Health.Health_Bar` (`self.HealthUI`)) (/ (`self.Health`) 1000.0)))

(event `/Game/VisualSandbox/Blueprints/Boss/BPI_BossFight.Attack`
  (bind _attack_pos (`self.Attack Pos`))
  (bind _returnvalue (`SceneComponent.K2_GetComponentLocation` _attack_pos))
  ; Attack
  (if (and (not (`self.IsAttacking?`)) (not (`self.isDead?`)))
    (`|PlayMontage` (`self.Mesh`) "/Game/MonsterForSurvivalGame/Animation/PBR/Beholder/Beholder_Attack01_ANIM_Montage.Beholder_Attack01_ANIM_Montage"
      (:`then`
        (set `self.IsAttacking?` true))
      (:`OnCompleted`
        (set `self.IsAttacking?` false))
      (:`OnNotifyBegin`
        (`|ExecutionSequence`
          (:`then_0`
            (bind (_outhit _returnvalue_2) (`KismetSystemLibrary.SphereTraceSingleForObjects` :`Start` _returnvalue :`End` (+ _returnvalue (* (`KismetMathLibrary.GetForwardVector` (`SceneComponent.K2_GetComponentRotation` _attack_pos)) 1500)) :`Radius` 90.0 :`ObjectTypes` (`|MakeArray` "ObjectTypeQuery3" :!type "EObjectTypeQuery Enum") :`DrawTime` 2.0))
            (if _returnvalue_2
              (`GameplayStatics.ApplyDamage` (`.HitActor` (`GameplayStatics.BreakHitResult` _outhit)) (`self.Damage`))))
          (:`then_1`
            (`GameplayStatics.PlayWorldCameraShake` "/Game/VisualSandbox/Blueprints/Boss/BP_BossAttackShake.BP_BossAttackShake_C" (`self.K2_GetActorLocation`) 0.0 3500.0))
          (:`then_2`
            (`NiagaraFunctionLibrary.SpawnSystemAtLocation` "/Game/Fab/DrapEffet/Texture/BossAttackEffect1.BossAttackEffect1" (`SceneComponent.K2_GetComponentLocation` (`self.Attack Pos`)) (struct) (1.0 1.0 1.0) true true "AutoRelease")
            (`GameplayStatics.PlaySoundAtLocation` "/Game/FreeModularMagicSFX/D1_Spell/Mono/SW_MagicWeapon_Summon_1.SW_MagicWeapon_Summon_1" (`self.K2_GetActorLocation`) (struct) 1.5 1.0 0.0 null null null null)))))))

(fn `UserConstructionScript`)