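; BP_Proj_Rocket is a rocket projectile that explodes on impact and can be leveled up.
; On impact it spawns an explosion at its location from its ExplosionType struct and radial force, crediting the instigator and ignoring the first player's character, then destroys itself.
; LevelUp rebuilds that struct with increased damage, minimum damage and inner and outer radii, keeping effects, falloff and noise settings unchanged.
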(fn `LevelUp`
  (bind (_explosion_type_explosionsound _explosion_type_explosionfx _explosion_type_explosiondamage _explosion_type_explosionmindamage _explosion_type_explosioninnerradius _explosion_type_explosionouterradius _explosion_type_damagefalloff _explosion_type_damagetypeclass _explosion_type_damagepreventionchannel _explosion_type_explosionnoiseloudness _explosion_type_explosionnoiserange _explosion_type_explosionnoisetag) (break `/Game/VisualSandbox/Blueprints/Structures/FExplosionData` (`self.Explosion Type`)))
  (set `self.Explosion Type` (make `/Game/VisualSandbox/Blueprints/Structures/FExplosionData` _explosion_type_explosionsound _explosion_type_explosionfx (+ _explosion_type_explosiondamage 50.0) (+ _explosion_type_explosionmindamage 10.0) (+ _explosion_type_explosioninnerradius 15.0) (+ _explosion_type_explosionouterradius 50.0) _explosion_type_damagefalloff _explosion_type_damagetypeclass _explosion_type_damagepreventionchannel _explosion_type_explosionnoiseloudness _explosion_type_explosionnoiserange _explosion_type_explosionnoisetag)))

(fn `On Impact`
  (params (`Impact Result` :type "HitResult Structure"))
  (`/Game/VisualSandbox/Blueprints/Utility/BP_UsefulFunctions.Spawn Explosion` (`self.K2_GetActorLocation`) (`self.Explosion Type`) (`|MakeArray` (`GameplayStatics.GetPlayerCharacter` 0) :!type "Actor Object Reference") self (`self.GetInstigatorController`) (`self.RadialForce`))
  (`self.K2_DestroyActor`))

(fn `UserConstructionScript`
  (`parent.UserConstructionScript`))